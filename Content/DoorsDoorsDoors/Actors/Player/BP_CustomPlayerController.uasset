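; Player controller for DoorsDoorsDoors that turns legacy input bindings into first-order movement, jumping and camera look for the controlled Character.
; Jump press and release call Jump and StopJumping on the pawn, each printing a debug message.
; Forward and right axes push input vectors along the character's forward and right vectors through its movement component, while look and turn axes add controller pitch and yaw.
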(event EventBeginPlay)

(event EventTick
  (params (DeltaSeconds :type Float%20%28single-precision%29)))

(event Input|ActionEvents|InputActionJump
  (params (Key :type Key%20Structure :default "None"))
  (bind _returnvalue (Pawn|GetControlledPawn))
  (:Pressed
    (bind _ascharacter (Utilities|Casting|CastToCharacter _returnvalue))
    (Character|Jump _ascharacter)
    (Development|PrintString "Jump"))
  (:Released
    (Utilities|Casting|CastToCharacter _returnvalue)
    (Character|StopJumping _ascharacter)
    (Development|PrintString "Stop Jump")))

(event Input|AxisEvents|InputAxisMoveForward/Backward
  (params (AxisValue :type Float%20%28single-precision%29))
  (bind _ascharacter (Utilities|Casting|CastToCharacter (Pawn|GetControlledPawn)))
  (Class|PawnMovementComponent|AddInputVector (Pawn|GetMovementComponent _ascharacter) (* (Transformation|GetActorForwardVector _ascharacter) AxisValue) false))

(event Input|AxisEvents|InputAxisLookUp
  (params (AxisValue :type Float%20%28single-precision%29))
  (Class|PlayerController|AddPitchInput AxisValue))

(event Input|AxisEvents|InputAxisTurn
  (params (AxisValue :type Float%20%28single-precision%29))
  (Class|PlayerController|AddYawInput AxisValue))

(event Input|AxisEvents|InputAxisMoveRight/Left
  (params (AxisValue :type Float%20%28single-precision%29))
  (bind _ascharacter (Utilities|Casting|CastToCharacter (Pawn|GetControlledPawn)))
  (Class|PawnMovementComponent|AddInputVector (Pawn|GetMovementComponent _ascharacter) (* (Transformation|GetActorRightVector _ascharacter) AxisValue) false))

(fn ConstructionScript)